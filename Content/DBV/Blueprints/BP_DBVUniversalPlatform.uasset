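; Configurable platform actor that can travel back and forth, spin or rock, and break apart when hit.
; While active, Tick shuttles it between its start and Destination along an unnormalized vector, and either rotates it continuously or, in balance mode, reverses rotation past an angle limit.
; If breakable, each overlap, throttled by a cooldown, advances through a mesh array of damage stages until the actor is destroyed.
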(event EventBeginPlay
  ;[1 1 1] Start Initialising Location and Breaking State
  (CallFunction|InitLocation)
  (CallFunction|InitBrokenFloor))

(event EventTick
  (params (DeltaSeconds :type Float%20%28single-precision%29))
  ;[1 1 1] If active, in every frame the parameters of movement and rotation are checked and updated
  (if (Variables|DBV|GetisActive)
    (CallFunction|MovePlatform DeltaSeconds)
    (if (Variables|DBV|Balance|GetisBalance)
      (CallFunction|BalancePlatform DeltaSeconds)
      (else
        (CallFunction|RotatePlatform DeltaSeconds)))))

(event Collision|EventActorBeginOverlap
  (params (OtherActor :type Actor%20Object%20Reference))
  ;[1 1 1] Whe the user hits a platform it will break it (unless the time has not been enough between overlaps)
  (if (CallFunction|CanBreakNow)
    (CallFunction|UpdateBrokenFloor)
    (Variables|DBV|BrokenFloor|SetWaiting true)
    (Utilities|FlowControl|Delay (Variables|DBV|BrokenFloor|GetCollisionInterval))
    (Variables|DBV|BrokenFloor|SetWaiting false)))

(fn ConstructionScript)

(fn MovePlatform
  (params (DeltaTime :type Float%20%28double-precision%29))
  (bind _returnvalue (Transformation|GetActorLocation))
  (bind _output_get (Variables|DBV|Movement|SetDistance (+ (Variables|DBV|Movement|GetDistance) (Math|Vector|Distance(Vector) (+ (* (Variables|DBV|Movement|GetVDirection) (Variables|DBV|Movement|GetVelocity) DeltaTime) _returnvalue) _returnvalue))))
  (Transformation|SetActorLocation (+ (* (Variables|DBV|Movement|GetVDirection) (Variables|DBV|Movement|GetVelocity) DeltaTime) _returnvalue) false false)
  (if (>= _output_get (Variables|DBV|Movement|GetMaximumDistance))
    (Variables|DBV|Movement|SetVDirection (* (Variables|DBV|Movement|GetVDirection) -1.0))
    (Variables|DBV|Movement|SetDistance 0.0)))

(fn RotatePlatform
  (params (DeltaTime :type Float%20%28double-precision%29))
  (Transformation|AddActorLocalRotation (* (Variables|DBV|Rotation|GetRotationVelocity) DeltaTime) false false))

(fn BalancePlatform
  (params (DeltaTime :type Float%20%28double-precision%29))
  (bind _maximumrotationdistance (Variables|DBV|Balance|GetMaximumRotationDistance))
  (bind _returnvalue (* _maximumrotationdistance -1.0))
  (bind _output_get (Variables|DBV|Rotation|SetRotationDistance (Math|Rotator|MakeRotator (+ (.roll (Variables|DBV|Rotation|GetRotationDistance)) (.roll (* (Variables|DBV|Rotation|GetRotationVelocity) DeltaTime))) (+ (.pitch (* (Variables|DBV|Rotation|GetRotationVelocity) DeltaTime)) (.pitch (Variables|DBV|Rotation|GetRotationDistance))) (+ (.yaw (* (Variables|DBV|Rotation|GetRotationVelocity) DeltaTime)) (.yaw (Variables|DBV|Rotation|GetRotationDistance))))))
  (Transformation|AddActorLocalRotation (Math|Rotator|MakeRotator (.roll (* (Variables|DBV|Rotation|GetRotationVelocity) DeltaTime)) (.pitch (* (Variables|DBV|Rotation|GetRotationVelocity) DeltaTime)) (.yaw (* (Variables|DBV|Rotation|GetRotationVelocity) DeltaTime))) false false)
  (if (Math|Boolean|ORBoolean (> (.roll _output_get) _maximumrotationdistance) (> (.pitch _output_get) _maximumrotationdistance) (> (.yaw _output_get) _maximumrotationdistance) (< (.roll _output_get) _returnvalue) (< (.pitch _output_get) _returnvalue) (< (.yaw _output_get) _returnvalue))
    (Variables|DBV|Rotation|SetRotationVelocity (* (Variables|DBV|Rotation|GetRotationVelocity) -1.0))
    (Variables|DBV|Rotation|SetRotationDistance "0, 0, 0")))

(fn InitBrokenFloor
  (if (Variables|DBV|BrokenFloor|GetcanBreakFloor)
    (Components|StaticMesh|SetStaticMesh (Variables|Default|GetStaticMesh) (Utilities|Array|Get(acopy) (Variables|DBV|BrokenFloor|GetSM_Floor)))
    (else
      (Collision|SetCollisionResponsetoChannel (Variables|Default|GetCollision) "ECC_Pawn" "ECR_Block"))))

(fn InitLocation
  (bind _returnvalue (Transformation|GetActorLocation))
  (bind _destination (Variables|DBV|Movement|GetDestination))
  (Variables|DBV|Movement|SetMaximumDistance (Math|Vector|Distance(Vector) _destination _returnvalue))
  (Variables|DBV|Movement|SetVDirection (- _destination _returnvalue)))

(fn UpdateBrokenFloor
  (bind _sm_floor (Variables|DBV|BrokenFloor|GetSM_Floor))
  (bind _result (Math|Integer|IncrementInt (Variables|DBV|BrokenFloor|GetCurrentPos))
    (:%20%20
      (if (> _result (Utilities|Array|Length _sm_floor))
        (Actor|DestroyActor)
        (else
          (Components|StaticMesh|SetStaticMesh (Variables|Default|GetStaticMesh) (Utilities|Array|Get(acopy) _sm_floor _result)))))))

(fn CanBreakNow
  (return (and (Variables|DBV|BrokenFloor|GetcanBreakFloor) (not (Variables|DBV|BrokenFloor|GetWaiting)))))