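; Enemy template that appears at the start of a spline, fires bullets on a looping timer and optionally patrols the spline.
; A timeline moves the body between points, scaling play rate by segment length for constant speed and facing each next point.
; At path end it hides, stops firing and can reappear after a delay.
; Damage routes to a health component, whose death event is bound to an empty handler.
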(event Custom|appear
  (Transformation|SetWorldLocation (Variables|Default|Getbody) (Spline|GetLocationatSplinePoint (Variables|Default|Gettrial) 0 "World") false false)
  (Development|SetHiddeninGame (Variables|Default|Getbody) false false)
  (Utilities|Time|SetTimerbyFunctionName 0 "fire" (Variables|Default|GetbulletInterval) true)
  (if (Variables|Default|GetdoPatrol)
    (CallFunction|Patrol)))

(event Custom|disappear
  (Development|SetHiddeninGame (Variables|Default|Getbody) true false)
  (Utilities|Time|ClearTimerbyFunctionName 0 "fire")
  (if (and (Variables|Default|GetdoPatrol) (Variables|Default|GetdoLoop))
    (Utilities|FlowControl|Delay (Variables|Default|GetloopInterval))
    (CallFunction|Appear)))

(event Custom|patrol
  (Variables|Default|SetpointNumber (Spline|GetNumberOfSplinePoints (Variables|Default|Gettrial)))
  (bind _output_get (Variables|Default|Setindex 1))
  (CallFunction|PrepareforNextPoint _output_get)
  (bind _alpha (Timeline|alpha PlayFromStart)
    (:Update
      (Transformation|SetWorldLocation (Variables|Default|Getbody) (Math|Vector|Lerp(Vector) (Variables|Default|GetoldPosition) (Variables|Default|GetnewPostion) _alpha) false false))
    (:Finished
      (if (|(a<(b-1)) (Variables|Default|Getindex) (Variables|Default|GetpointNumber))
        (bind _result (Math|Integer|IncrementInt (Variables|Default|Getindex))
          (:%20%20
            (CallFunction|PrepareforNextPoint _result)
            (Timeline|alpha PlayFromStart)))
        (else
          (CallFunction|Disappear))))))

(event Custom|death)

(event Game|Damage|EventAnyDamage
  (params (Damage :type Float%20%28single-precision%29) (DamageType :type Damage%20Type%20Object%20Reference) (InstigatedBy :type Controller%20Object%20Reference) (DamageCauser :type Actor%20Object%20Reference))
  (Default|AnyDamge (Variables|Default|GetBP_HealthComponent) Damage))

(event EventBeginPlay
  (EventDispatchers|BindEventtoOnDeath (Variables|Default|GetBP_HealthComponent) (delegate Custom|death)))

(fn ConstructionScript
  (Development|SetHiddeninGame (Variables|Default|Getbody) false false)
  (Variables|/Game/Interactables/EnemyTemplate/BP_HealthComponent.BP_HealthComponent_C|SetBlood (Variables|Default|GetBP_HealthComponent) (Variables|Default|GetBlood))
  (Transformation|SetWorldLocation (Variables|Default|Getbody) (Spline|GetLocationatSplinePoint (Variables|Default|Gettrial) 0 "World") false false))

(fn PrepareforNextPoint
  (params (nextPointIndex :type Integer))
  (bind _output_get (Variables|Default|SetoldPosition (Transformation|GetWorldLocation (Variables|Default|Getbody))))
  (bind _output_get_2 (Variables|Default|SetnewPostion (Spline|GetLocationatSplinePoint (Variables|Default|Gettrial) nextPointIndex "World")))
  (Transformation|SetWorldRotation (Variables|Default|Getbody) (Math|Rotator|FindLookatRotation _output_get _output_get_2) false false)
  (Components|Timeline|SetPlayRate (Variables|CameraModifier|GetAlpha) (/ (Variables|Default|Getspeed) (Math|Vector|VectorLength (- _output_get_2 _output_get)))))

(fn Fire
  (Game|SpawnActorfromClass "/Game/Interactables/EnemyTemplate/BP_Bullet.BP_Bullet_C" (Transformation|GetWorldTransform (Variables|Default|GetbulletStartPoint)) "AdjustIfPossibleButAlwaysSpawn" "MultiplyWithRoot" 0 (Variables|Default|GetbulletDamage) (Variables|Default|GetbulletSpeed) (Math|Vector|GetForwardVector (Variables|Default|GetbulletStartPoint)) 0))