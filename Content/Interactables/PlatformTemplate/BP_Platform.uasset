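; Platform template that travels along a Trial spline, either continuously or triggered by a BP_PlatformingCharacter.
; BeginPlay snaps movable platforms to the spline start and scales the Alpha timeline's play rate by Speed over spline length.
; Non-triggerable platforms call Move every Tick; triggerable ones loop forward on Box overlap and reverse without looping on exit.
; Timeline updates set position along the spline and follow only its yaw.
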(event OnComponentBeginOverlap(Box)
  (params (OverlappedComponent :type Primitive%20Component%20Object%20Reference) (OtherActor :type Actor%20Object%20Reference) (OtherComp :type Primitive%20Component%20Object%20Reference) (OtherBodyIndex :type Integer) (bFromSweep :type Boolean) (SweepResult :type Hit%20Result%20Structure%20%28by%20ref%29))
  (bind _asbp_platforming_character (Utilities|Casting|CastToBP_PlatformingCharacter OtherActor))
  (Utilities|IsValid _asbp_platforming_character
    (:Is%20Valid
      (if (Variables|Default|GetMovable)
        (if (Variables|Default|GetTriggerable)
          (CallFunction|Move))))))

(event OnComponentEndOverlap(Box)
  (params (OverlappedComponent :type Primitive%20Component%20Object%20Reference) (OtherActor :type Actor%20Object%20Reference) (OtherComp :type Primitive%20Component%20Object%20Reference) (OtherBodyIndex :type Integer))
  (bind _asbp_platforming_character (Utilities|Casting|CastToBP_PlatformingCharacter OtherActor))
  (Utilities|IsValid _asbp_platforming_character
    (:Is%20Valid
      (if (Variables|Default|GetMovable)
        (if (Variables|Default|GetTriggerable)
          (CallFunction|Reverse))))))

(event Custom|Move
  (bind _platform (Variables|Default|Getplatform))
  (bind _returnvalue (Transformation|GetWorldRotation _platform))
  (Components|Timeline|SetLooping (Variables|CameraModifier|GetAlpha) true)
  (bind _alpha (Timeline|alpha Play)
    (:Update
      (Transformation|SetWorldLocationAndRotation (Variables|Default|Getplatform) (.location (Spline|GetTransformatDistanceAlongSpline (Variables|Default|Gettrial) (* _alpha (Variables|Default|GetSplineLength)) "World" false)) (Math|Rotator|MakeRotator (.roll _returnvalue) (.pitch _returnvalue) (.yaw (.rotation (Spline|GetTransformatDistanceAlongSpline (Variables|Default|Gettrial) (* _alpha (Variables|Default|GetSplineLength)) "World" false)))) false false))))

(event Custom|reverse
  (bind _platform (Variables|Default|Getplatform))
  (bind _returnvalue (Transformation|GetWorldRotation _platform))
  (Components|Timeline|SetLooping (Variables|CameraModifier|GetAlpha) false)
  (bind _alpha (Timeline|alpha Reverse)
    (:Update
      (Transformation|SetWorldLocationAndRotation (Variables|Default|Getplatform) (.location (Spline|GetTransformatDistanceAlongSpline (Variables|Default|Gettrial) (* _alpha (Variables|Default|GetSplineLength)) "World" false)) (Math|Rotator|MakeRotator (.roll _returnvalue) (.pitch _returnvalue) (.yaw (.rotation (Spline|GetTransformatDistanceAlongSpline (Variables|Default|Gettrial) (* _alpha (Variables|Default|GetSplineLength)) "World" false)))) false false))))

(event EventBeginPlay
  (if (Variables|Default|GetMovable)
    (Transformation|SetWorldLocation (Variables|Default|Getplatform) (Spline|GetLocationatSplinePoint (Variables|Default|Gettrial) 0 "World") false false)
    (bind _output_get (Variables|Default|SetSplineLength (Spline|GetSplineLength (Variables|Default|Gettrial))))
    (Components|Timeline|SetPlayRate (Variables|CameraModifier|GetAlpha) (/ (Variables|Default|GetSpeed) _output_get))))

(event EventTick
  (params (DeltaSeconds :type Float%20%28single-precision%29))
  (if (Variables|Default|GetMovable)
    (if (not (Variables|Default|GetTriggerable))
      (CallFunction|Move))))

(fn ConstructionScript)